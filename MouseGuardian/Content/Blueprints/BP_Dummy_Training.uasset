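; Training dummy actor that takes damage and shows its health on a floating widget bar.
; On begin play it caches the WB_DummyHealthBar widget and refreshes it through the BPCPlayerStats component.
; Any damage prints a debug string and removes a fixed amount of health through that component, ignoring the incoming damage value.
; Each tick turns the health bar widget to face the player camera.
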(event EventBeginPlay
  (bind _aswb_dummy_health_bar (Utilities|Casting|CastToWB_DummyHealthBar (UserInterface|GetWidget (Variables|Default|GetHealth%20Bar%20Widget))))
  (Variables|Default|SetHealth%20Bar%20Widget%20BP _aswb_dummy_health_bar)
  (Default|UpdateHealthBar (Variables|Default|GetBPC_PlayerStats)))

(event Collision|EventActorBeginOverlap
  (params (OtherActor :type Actor%20Object%20Reference)))

(event EventTick
  (params (DeltaSeconds :type Float%20%28single-precision%29))
  (Transformation|SetWorldRotation (Variables|Default|GetHealth%20Bar%20Widget) (Math|Rotator|FindLookatRotation (Transformation|GetWorldLocation (Variables|Default|GetHealth%20Bar%20Widget)) (Transformation|GetWorldLocation (Variables|/Script/Engine.PlayerCameraManager|GetTransformComponent (Game|GetPlayerCameraManager 0)))) false false))

(event Game|Damage|EventAnyDamage
  (params (Damage :type Float%20%28single-precision%29) (DamageType :type Damage%20Type%20Object%20Reference) (InstigatedBy :type Controller%20Object%20Reference) (DamageCauser :type Actor%20Object%20Reference))
  (Development|PrintString "damageeeeeee")
  (Default|DecreaseHealth (Variables|Default|GetBPC_PlayerStats) 1e+01))

(fn ConstructionScript)