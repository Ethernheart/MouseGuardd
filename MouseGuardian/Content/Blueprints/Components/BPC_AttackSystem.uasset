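; Actor component that gives BP_ThirdPersonCharacter a two-hit sword combo and melee damage.
; Attack input, gated by CanAttack, plays the montage for the current AttackIndex, buffering presses made mid-attack.
; SwordComboAttack continues a buffered combo or resets it.
; StartSwordTrace and StopSwordTrace control a looping timer that sphere-traces between the sword points, damaging "Damagable"-tagged pawns behind a delayed DoOnce to limit repeat hits.
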(event Custom|Sword%20Attack
  ;[1 1 1] Combo system
  ;;[1 1 1] Sword Attack
  (if (Variables|Default|GetIs%20Attacking)
    (Variables|Default|SetSave%20Attack true)
    (else
      (Variables|Default|SetIs%20Attacking true)
      (switch int (Variables|Default|GetAttack%20Index)
        (:0
          (CallFunction|Attack1))
        (:1
          (CallFunction|Attack2))))))

(event Custom|Sword%20Combo%20Attack
  ;[1 1 1] Combo system
  ;;[1 1 1] Combo
  (if (Variables|Default|GetSave%20Attack)
    (Variables|Default|SetSave%20Attack false)
    (switch int (Variables|Default|GetAttack%20Index)
      (:0
        (CallFunction|Attack1))
      (:1
        (CallFunction|Attack2)))
    (else
      (CallFunction|StopCombo))))

(event Custom|Stop%20Combo
  ;[1 1 1] Combo system
  ;;[1 1 1] Stop Combo
  (Variables|Default|SetIs%20Attacking false)
  (Variables|Default|SetAttack%20Index 0))

(event Custom|Attack2
  ;[1 1 1] Combo system
  ;;[1 1 1] Attack 2
  (Utilities|FlowControl|DoOnce false :!label _label
    (:Completed
      (Utilities|FlowControl|Delay 0.1)
      (Animation|Montage|PlayMontage (Variables|Default|GetCharacter%20Mesh) "/Game/Characters/Mouse/Animations/Attack_Animation/Attack2_Mouse_Montage.Attack2_Mouse_Montage"
        (:then
          (Variables|Default|SetAttack%20Index 2)
          (goto _label Reset))))))

(event Custom|Start%20Sword%20Trace
  ;[1 1 1] Sword Trace
  (bind _returnvalue (Utilities|Time|SetTimerbyEvent (delegate Custom|Sword%20Trace%20Loop) 0.01 true))
  (Variables|Default|SetSwordTraceLoop _returnvalue))

(event Custom|Sword%20Trace%20Loop
  (bind _character_bp (Variables|Default|GetCharacter%20BP))
  ;[1 1 1] Sword Trace
  (bind (_outhit _returnvalue) (Collision|SphereTraceForObjects (Transformation|GetWorldLocation (Variables|/Game/ThirdPerson/Blueprints/Charater/BP_ThirdPersonCharacter.BP_ThirdPersonCharacter_C|GetSword%20Top%20Point _character_bp)) (Transformation|GetWorldLocation (Variables|/Game/ThirdPerson/Blueprints/Charater/BP_ThirdPersonCharacter.BP_ThirdPersonCharacter_C|GetSword%20Bottom%20Point _character_bp)) 0.0 (Utilities|Array|MakeArray "ObjectTypeQuery3") false 0 "None"))
  (if _returnvalue
    (if (Actor|ActorHasTag (.HitActor (Collision|BreakHitResult _outhit)) "Damagable")
      (Utilities|FlowControl|DoOnce false :!label _label
        (:Completed
          (Game|Damage|ApplyDamage (.HitActor (Collision|BreakHitResult _outhit)) 1e+01 0 0)
          (Utilities|FlowControl|Delay 0.5)
          (goto _label Reset))))))

(event Custom|Stop%20Sword%20Trace
  ;[1 1 1] Sword Trace
  (Utilities|Time|ClearandInvalidateTimerbyHandle (Variables|Default|GetSwordTraceLoop)))

(event Custom|Attack%201
  ;[1 1 1] Combo system
  ;;[1 1 1] Attack 1
  (Utilities|FlowControl|DoOnce false :!label _label
    (:Completed
      (Utilities|FlowControl|Delay 0.1)
      (Animation|Montage|PlayMontage (Variables|Default|GetCharacter%20Mesh) "/Game/Characters/Mouse/Animations/Attack_Animation/Attack1_Mouse_Montage.Attack1_Mouse_Montage"
        (:then
          (Variables|Default|SetAttack%20Index 1)
          (goto _label Reset))))))

(event Input|EnhancedActionEvents|EnhancedInputActionIA_Attack
  (params (ActionValue :type Boolean) (ElapsedSeconds :type Float%20%28double-precision%29) (TriggeredSeconds :type Float%20%28double-precision%29) (InputAction :type Input%20Action%20Object%20Reference :default "/Game/ThirdPerson/Input/Actions/IA_Attack.IA_Attack"))
  ;[1 1 1] Combo system
  ;;[1 1 1] Attack Input
  (:Started
    (if (Variables|Default|GetCan%20Attack)
      (CallFunction|SwordAttack))))

(event EventBeginPlay
  ;[1 1 1] Get Character Mesh
  (bind _asbp_third_person_character (Utilities|Casting|CastToBP_ThirdPersonCharacter (Components|GetOwner)))
  (Variables|Default|SetCharacter%20BP _asbp_third_person_character)
  (Variables|Default|SetCharacter%20Mesh (Variables|/Script/Engine.Character|GetMesh _asbp_third_person_character)))