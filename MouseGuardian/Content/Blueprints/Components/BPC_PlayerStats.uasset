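; Actor component that holds health and mana stats for its owning BP_ThirdPersonCharacter or BP_DummyTraining.
; BeginPlay caches the owner and sets IsPlayer, though bar updates always go through the player character's HUD widget.
; Health and mana changes are clamped, then pushed to HUD bars and text; DecreaseHealth returns whether health is depleted.
; DecreaseMana subtracts ManaRestoration, and both mana functions flag IsManaOwerflow at maximum.
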(event EventBeginPlay
  (bind _asbp_third_person_character (Utilities|Casting|CastToBP_ThirdPersonCharacter (Components|GetOwner))
    (:then
      (Variables|Default|SetPlayer%20Character%20BP _asbp_third_person_character)
      (Variables|Default|SetIs%20Player true))
    (:CastFailed
      (bind _asbp_dummy_training (Utilities|Casting|CastToBP_DummyTraining (Components|GetOwner)))
      (Variables|Default|SetDummy%20BP _asbp_dummy_training)
      (Variables|Default|SetIs%20Player false))))

(event EventTick
  (params (DeltaSeconds :type Float%20%28single-precision%29)))

(fn DecreaseHealth
  (params (Taken%20Damage :type Float%20%28double-precision%29))
  (Variables|Health|SetCurrentHealth (Math|Float|Clamp(Float) (- (Variables|Health|GetCurrentHealth) Taken%20Damage) 0.0 (Variables|Health|GetMaxHealth)))
  (HUD|UpdateHealthBar)
  (if (<= (Variables|Health|GetCurrentHealth) 0.0)
    (return true)
    (else
      (return false))))

(fn IncreaseHealth
  (params (Added%20Health :type Float%20%28double-precision%29))
  (Variables|Health|SetCurrentHealth (Math|Float|Clamp(Float) (+ (Variables|Health|GetCurrentHealth) Added%20Health) 0.0 (Variables|Health|GetMaxHealth)))
  (HUD|UpdateHealthBar))

(fn UpdateHealthBar
  (Progress|SetPercent (Variables|/Game/Widgets/WB_HUD.WB_HUD_C|GetHealthBar (Variables|/Game/ThirdPerson/Blueprints/Charater/BP_ThirdPersonCharacter.BP_ThirdPersonCharacter_C|GetHUD%20Widget (Variables|Default|GetPlayer%20Character%20BP))) (/ (Variables|Health|GetCurrentHealth) (Variables|Health|GetMaxHealth)))
  (Rendering|Components|TextRender|SetText (Variables|/Game/Widgets/WB_HUD.WB_HUD_C|GetHealthText (Variables|/Game/ThirdPerson/Blueprints/Charater/BP_ThirdPersonCharacter.BP_ThirdPersonCharacter_C|GetHUD%20Widget (Variables|Default|GetPlayer%20Character%20BP))) (Utilities|Text|ToText(Float) (Variables|Health|GetCurrentHealth) "HalfToEven")))

(fn IncreaseMana
  (params (B :type Float%20%28double-precision%29))
  (Variables|Mana|SetCurrentMana (Math|Float|Clamp(Float) (+ (Variables|Mana|GetCurrentMana) B) 0.0 (Variables|Mana|GetMaxMana)))
  (HUD|UpdateManaBar)
  (Variables|Default|SetIs%20Mana%20Owerflow (>= (Variables|Mana|GetCurrentMana) (Variables|Mana|GetMaxMana)))
  (return))

(fn DecreaseMana
  (Variables|Mana|SetCurrentMana (Math|Float|Clamp(Float) (- (Variables|Mana|GetCurrentMana) (Variables|Mana|GetManaRestoration)) 0.0 (Variables|Mana|GetMaxMana)))
  (HUD|UpdateManaBar)
  (Variables|Default|SetIs%20Mana%20Owerflow (not (< (Variables|Mana|GetCurrentMana) (Variables|Mana|GetMaxMana)))))

(fn UpdateManaBar
  (Progress|SetPercent (Variables|/Game/Widgets/WB_HUD.WB_HUD_C|GetManaBar (Variables|/Game/ThirdPerson/Blueprints/Charater/BP_ThirdPersonCharacter.BP_ThirdPersonCharacter_C|GetHUD%20Widget (Variables|Default|GetPlayer%20Character%20BP))) (/ (Variables|Mana|GetCurrentMana) (Variables|Mana|GetMaxMana)))
  (Rendering|Components|TextRender|SetText (Variables|/Game/Widgets/WB_HUD.WB_HUD_C|GetManaText (Variables|/Game/ThirdPerson/Blueprints/Charater/BP_ThirdPersonCharacter.BP_ThirdPersonCharacter_C|GetHUD%20Widget (Variables|Default|GetPlayer%20Character%20BP))) (Utilities|Text|ToText(Float) (Variables|Mana|GetCurrentMana) "HalfToEven")))