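; Health component, named for the training dummy, that tracks and clamps its owner's current health.
; BeginPlay casts the owner to the third-person character or the training dummy, storing the reference and an IsPlayer flag.
; Decrease and increase functions refresh the health bar, with decrease also returning whether health reached zero.
; The bar update writes percent and text only through the dummy's widget, even when the owner is the player.
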(event EventBeginPlay
  (bind _asbp_third_person_character (Utilities|Casting|CastToBP_ThirdPersonCharacter (Components|GetOwner))
    (:then
      (Variables|Default|SetPlayer%20Character%20BP _asbp_third_person_character)
      (Variables|Default|SetIs%20Player true))
    (:CastFailed
      (bind _asbp_dummy_training (Utilities|Casting|CastToBP_DummyTraining (Components|GetOwner)))
      (Variables|Default|SetDummy%20BP _asbp_dummy_training)
      (Variables|Default|SetIs%20Player false))))

(event EventTick
  (params (DeltaSeconds :type Float%20%28single-precision%29)))

(fn DecreaseHealth
  (params (Taken%20Damage :type Float%20%28double-precision%29))
  (Variables|Health|SetCurrentHealth (Math|Float|Clamp(Float) (- (Variables|Health|GetCurrentHealth) Taken%20Damage) 0.0 (Variables|Health|GetMaxHealth)))
  (HUD|UpdateHealthBar)
  (if (<= (Variables|Health|GetCurrentHealth) 0.0)
    (return true)
    (else
      (return false))))

(fn IncreaseHealth
  (params (Added%20Health :type Float%20%28double-precision%29))
  (Variables|Health|SetCurrentHealth (Math|Float|Clamp(Float) (+ (Variables|Health|GetCurrentHealth) Added%20Health) 0.0 (Variables|Health|GetMaxHealth)))
  (HUD|UpdateHealthBar))

(fn UpdateHealthBar
  (Progress|SetPercent (Variables|/Game/Widgets/WB_HealthBar.WB_HealthBar_C|GetHealthBar_Enemy (Variables|/Game/Actors/Dummy/BP_DummyTraining.BP_DummyTraining_C|GetHealth%20Bar%20Widget%20BP (Variables|Default|GetDummy%20BP))) (/ (Variables|Health|GetCurrentHealth) (Variables|Health|GetMaxHealth)))
  (Rendering|Components|TextRender|SetText (Variables|/Game/Widgets/WB_HealthBar.WB_HealthBar_C|GetHealthTextEnemy (Variables|/Game/Actors/Dummy/BP_DummyTraining.BP_DummyTraining_C|GetHealth%20Bar%20Widget%20BP (Variables|Default|GetDummy%20BP))) (Utilities|Text|ToText(Float) (Variables|Health|GetCurrentHealth) "HalfToEven")))