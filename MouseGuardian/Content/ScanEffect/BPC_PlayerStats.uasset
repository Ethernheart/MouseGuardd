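; Player stats actor component that tracks health for BP_ThirdPersonCharacter and keeps its HUD in sync.
; On BeginPlay it casts and caches the owning character.
; Decrease and increase functions clamp health between zero and max, then refresh the health bar percent and text on the character's HUD widget.
; DecreaseHealth also returns whether health has reached zero, signalling death to the caller.
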(event EventBeginPlay
  (bind _asbp_third_person_character (Utilities|Casting|CastToBP_ThirdPersonCharacter (Components|GetOwner)))
  (Variables|Default|SetPlayer%20Character%20BP _asbp_third_person_character))

(event EventTick
  (params (DeltaSeconds :type Float%20%28single-precision%29)))

(fn DecreaseHealth
  (params (Taken%20Damage :type Float%20%28double-precision%29))
  (Variables|Health|SetCurrentHealth (Math|Float|Clamp(Float) (- (Variables|Health|GetCurrentHealth) Taken%20Damage) 0.0 (Variables|Health|GetMaxHealth)))
  (HUD|UpdateHealthBar)
  (if (<= (Variables|Health|GetCurrentHealth) 0.0)
    (return true)
    (else
      (return false))))

(fn IncreaseHealth
  (params (Added%20Health :type Float%20%28double-precision%29))
  (Variables|Health|SetCurrentHealth (Math|Float|Clamp(Float) (+ (Variables|Health|GetCurrentHealth) Added%20Health) 0.0 (Variables|Health|GetMaxHealth)))
  (HUD|UpdateHealthBar))

(fn UpdateHealthBar
  (bind _player_character_bp (Variables|Default|GetPlayer%20Character%20BP))
  (bind _hud_widget (Variables|/Game/ThirdPerson/Blueprints/Charater/BP_ThirdPersonCharacter.BP_ThirdPersonCharacter_C|GetHUD%20Widget _player_character_bp))
  (Progress|SetPercent (Variables|/Game/ScanEffect/WB_HUD.WB_HUD_C|GetHealthBar _hud_widget) (/ (Variables|Health|GetCurrentHealth) (Variables|Health|GetMaxHealth)))
  (Rendering|Components|TextRender|SetText (Variables|/Game/ScanEffect/WB_HUD.WB_HUD_C|GetHealthText _hud_widget) (Utilities|Text|ToText(Float) (Variables|Health|GetCurrentHealth) "HalfToEven")))